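; Behavior Tree task that moves a BP_AI pawn to the next point on its patrol path spline, one point per execution.
; After each move, successful or failed, UpdatePointIndex advances the stored index, wrapping on closed loops or ping-ponging on open splines, and the task reports success.
; It fails without a valid spline, stalls unfinished if the BP_AI cast fails, and stops movement on abort.
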(event `self.ReceiveAbortAI`
  (params (OwnerController :type "AIController Object Reference") (ControlledPawn :type "Pawn Object Reference"))
  (`Controller.StopMovement` OwnerController)
  (`self.FinishAbort`))

(event `self.ReceiveExecuteAI`
  (params (OwnerController :type "AIController Object Reference") (ControlledPawn :type "Pawn Object Reference"))
  (bind _asbp_ai (cast `/Game/AI/BP_AI` ControlledPawn))
  (bind _output_get (set `self.AI` _asbp_ai))
  (bind _spline (`/Game/AI/BP_PatrolPath.Spline` (`/Game/AI/BP_AI.BP_PatrolPath` _output_get)))
  (`/Engine/EditorBlueprintResources/StandardMacros.IsValid` _spline
    (:`Is Valid`
      (set `self.Spline` _spline)
      (`|AIMoveTo` (`self.AI`) (`SplineComponent.GetLocationAtSplinePoint` (`self.Spline`) (`self.PointIndex`) "World") null 50.0
        (:`OnSuccess`
          _)
        (:`OnFail`
          _))
      (`self.UpdatePointIndex`)
      (`self.FinishExecute` true))
    (:`Is Not Valid`
      (`self.FinishExecute` false))))

(fn `UpdatePointIndex`
  (if (`self.ReverseDirection`)
    (if (<= (`self.PointIndex`) 0)
      (set `self.PointIndex` 0)
      (set `self.ReverseDirection` false)
      (else
        (`/Engine/EditorBlueprintResources/StandardMacros.DecrementInt` (`self.PointIndex`))))
    (elif (>= (`self.PointIndex`) (- (`SplineComponent.GetNumberOfSplinePoints` (`self.Spline`)) 1))
      (if (`SplineComponent.IsClosedLoop` (`self.Spline`))
        (set `self.PointIndex` 0)
        (else
          (set `self.ReverseDirection` true)
          (set `self.PointIndex` (- (`SplineComponent.GetNumberOfSplinePoints` (`self.Spline`)) 2))))
      (else
        (`/Engine/EditorBlueprintResources/StandardMacros.IncrementInt` (`self.PointIndex`))))))