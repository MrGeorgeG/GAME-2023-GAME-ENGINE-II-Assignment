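; AI controller for BP_AI pawns that starts their behavior tree on possession and feeds it sight and noise perception.
; Perception updates set investigation state and location for "Noise" stimuli, tinting the mesh red, and treat all other stimuli as CanSeePlayer.
; A looping UpdateTarget timer takes the first sighted actor as blackboard target and tints the mesh yellow, clearing it beyond a fixed distance.
; Patrol-path setup nodes are unconnected.
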(event `self.ReceivePossess`
  (params (PossessedPawn :type "Pawn Object Reference"))
  (bind _asbp_ai (cast `/Game/AI/BP_AI` PossessedPawn))
  (set `self.MyPawn` _asbp_ai)
  (`self.RunBehaviorTree` "/Game/AI/Tack/BP_AIBT.BP_AIBT")
  (`KismetSystemLibrary.K2_SetTimer` null "UpdateTarget" 0.5 true))

(event `self.AIPerception.OnPerceptionUpdated`
  (params (UpdatedActors :type "Array of Actor Object Reference (by ref)"))
  ;[1 1 1] Gun
  (for _array_element UpdatedActors
    (bind _info (`AIPerceptionComponent.GetActorsPerception` (`self.AIPerception`) _array_element))
    (for _array_element_2 (`.LastSensedStimuli` (break `ActorPerceptionBlueprintInfo` _info))
      (bind _returnvalue (`PrimitiveComponent.CreateDynamicMaterialInstance` (`Character.Mesh` (`self.MyPawn`)) 0 "/Game/AI/M_Color.M_Color" "None"))
      (`self.EnableInput` (`GameplayStatics.GetPlayerController` 0))
      (bind (_age _expirationage _strength _stimuluslocation _receiverlocation _tag _bsuccessfullysensed) (break `AIStimulus` _array_element_2))
      (if (== _tag "Noise")
        (`BlackboardComponent.SetValueAsBool` (`AIBlueprintHelperLibrary.GetBlackboard` null) "IsInvestigating" _bsuccessfullysensed)
        (`BlackboardComponent.SetValueAsVector` (`AIBlueprintHelperLibrary.GetBlackboard` null) "TargetLocation" _stimuluslocation)
        (`MaterialInstanceDynamic.SetVectorParameterValue` _returnvalue "Color" (struct :`R` 1.0 :`G` 0.028959 :`B` 0.092671 :`A` 1.0))
        (else
          (`BlackboardComponent.SetValueAsBool` (`AIBlueprintHelperLibrary.GetBlackboard` null) "CanSeePlayer" _bsuccessfullysensed))))))

(event `self.AIPerception.OnTargetPerceptionUpdated`
  (params (Actor :type "Actor Object Reference") (Stimulus :type "AIStimulus Structure")))

(fn `UpdateTarget`
  (bind _returnvalue (`PrimitiveComponent.CreateDynamicMaterialInstance` (`Character.Mesh` (`self.MyPawn`)) 0 "/Game/AI/M_Color.M_Color" "None"))
  (`self.EnableInput` (`GameplayStatics.GetPlayerController` 0))
  (bind _output_get (set `self.ActorArray` (`AIPerceptionComponent.GetKnownPerceivedActors` (`self.AIPerception`) "/Script/AIModule.AISense_Sight")))
  (for _array_element _output_get
    (if (`KismetMathLibrary.ClassIsChildOf` (`GameplayStatics.GetObjectClass` _array_element) "/Script/Engine.Actor")
      (`KismetArrayLibrary.Array_AddUnique` (`self.TargetArr`) _array_element)))
  (if (> (`KismetArrayLibrary.Array_Length` (`self.TargetArr`)) 0)
    (set `self.Target` (`|GetArrayItem` (`self.TargetArr`)))
    (`self.Blackboard`
      (:`then`
        (if (> (`self.GetDistanceTo` (`self.K2_GetPawn`) (`self.Target`)) 500.0)
          (`BlackboardComponent.SetValueAsObject` (`self.Blackboard`) (`self.TargetKey`) null)
          (`KismetArrayLibrary.Array_Clear` (`self.TargetArr`))
          (else
            (`KismetSystemLibrary.PrintString` "gg2")
            (`MaterialInstanceDynamic.SetVectorParameterValue` _returnvalue "Color" (struct :`R` 0.657495 :`G` 0.6875 :`B` 0.056535 :`A` 1.0))
            (`BlackboardComponent.SetValueAsObject` (`self.Blackboard`) (`self.TargetKey`) (`self.Target`)))))
      (:`else`))))

(fn `UserConstructionScript`)